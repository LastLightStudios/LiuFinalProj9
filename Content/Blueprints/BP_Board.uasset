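; Grid board actor for a chess-like game that spawns tiles and units and handles click-to-move.
; ResetMap clears the board, then rebuilds floors, borders, obstacles, Grunts, Bishops and Rooks from two sample integer arrays.
; Helpers convert between index, coord and world location; IndexToCoord divides by Height, so only square boards map correctly.
; Click selects a unit, then moves it to any placeable, unoccupied tile, without movement rules.
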(event EventBeginPlay)

(event Collision|EventActorBeginOverlap
  (params (OtherActor :type Actor%20Object%20Reference)))

(event EventTick
  (params (DeltaSeconds :type Float%20%28single-precision%29)))

(fn ConstructionScript)

(fn CoordtoIndex
  (params (Coord :type Coord%20Structure))
  (return (+ (.x Coord) (* (.y Coord) (Variables|Default|GetWidth)))))

(fn IndextoCoord
  (params (Index :type Integer))
  (return (Utilities|Struct|MakeCoord (Math|Integer|%(Integer) Index (Variables|Default|GetWidth)) (/ Index (Variables|Default|GetHeight)))))

(fn ResetMap
  (bind _tilesize (Variables|Default|GetTileSize))
  (bind _returnvalue (/ _tilesize 2))
  (bind _returnvalue_2 (Math|Conversions|ToFloat(Integer) _returnvalue))
  (CallFunction|ClearMap)
  ;[1 1 1] Creating the Board
  (for (_array_element _array_index) (Variables|Default|GetSampleBoardArray)
    (switch int _array_element
      (:Default
        (Development|PrintString "Error in Sample Array"))
      (:0
        ;;[1 1 1] FIND OUT HOW TO MAKE THIS A SELECT
        (bind _returnvalue_3 (Game|SpawnActorfromClass "/Game/Blueprints/TileTypes/Floor.Floor_C" (Math|Transform|MakeTransform (CallFunction|CoordtoActualLocation (CallFunction|IndextoCoord _array_index)) "0, 0, 0" "1,1,1") "Undefined" 0 (CallFunction|IndextoCoord _array_index) 0))
        (Utilities|Array|Add (Variables|Default|GetTileArray) _returnvalue_3))
      (:1
        (bind _returnvalue_4 (Game|SpawnActorfromClass "/Game/Blueprints/TileTypes/Border.Border_C" (Math|Transform|MakeTransform (CallFunction|CoordtoActualLocation (CallFunction|IndextoCoord _array_index)) "0, 0, 0" "1,1,1") "Undefined" 0 (CallFunction|IndextoCoord _array_index) 0))
        (Utilities|Array|Add (Variables|Default|GetTileArray) _returnvalue_4))
      (:2
        (bind _returnvalue_5 (Game|SpawnActorfromClass "/Game/Blueprints/TileTypes/Obstacle.Obstacle_C" (Math|Transform|MakeTransform (CallFunction|CoordtoActualLocation (CallFunction|IndextoCoord _array_index)) "0, 0, 0" "1,1,1") "Undefined" 0 (CallFunction|IndextoCoord _array_index) 0))
        (Utilities|Array|Add (Variables|Default|GetTileArray) _returnvalue_5))))
  ;[1 1 1] Placing units
  (for (_array_element_2 _array_index_2) (Variables|Default|GetSampleUnitArray)
    (switch int _array_element_2
      (:Default
        (Development|PrintString "Error in Sample Unit Array"))
      (:1
        (bind _returnvalue_6 (Game|SpawnActorfromClass "/Game/Blueprints/UnitTypes/Grunt.Grunt_C" (Math|Transform|MakeTransform (Math|Vector|MakeVector (+ (.x (CallFunction|CoordtoActualLocation (CallFunction|IndextoCoord _array_index_2))) _returnvalue_2) (+ (.y (CallFunction|CoordtoActualLocation (CallFunction|IndextoCoord _array_index_2))) _returnvalue_2) (.z (CallFunction|CoordtoActualLocation (CallFunction|IndextoCoord _array_index_2)))) "0, 0, 0" "1,1,1") "Undefined" 0 (CallFunction|IndextoCoord _array_index_2) 0))
        (Utilities|Array|Add (Variables|Default|GetUnitArray) _returnvalue_6))
      (:2
        (bind _returnvalue_7 (Game|SpawnActorfromClass "/Game/Blueprints/UnitTypes/Bishop.Bishop_C" (Math|Transform|MakeTransform (Math|Vector|MakeVector (+ (.x (CallFunction|CoordtoActualLocation (CallFunction|IndextoCoord _array_index_2))) _returnvalue_2) (+ (.y (CallFunction|CoordtoActualLocation (CallFunction|IndextoCoord _array_index_2))) _returnvalue_2) (.z (CallFunction|CoordtoActualLocation (CallFunction|IndextoCoord _array_index_2)))) "0, 0, 0" "1,1,1") "Undefined" 0 (CallFunction|IndextoCoord _array_index_2) 0))
        (Utilities|Array|Add (Variables|Default|GetUnitArray) _returnvalue_7))
      (:3
        (bind _returnvalue_8 (Game|SpawnActorfromClass "/Game/Blueprints/UnitTypes/Rook.Rook_C" (Math|Transform|MakeTransform (Math|Vector|MakeVector (+ (.x (CallFunction|CoordtoActualLocation (CallFunction|IndextoCoord _array_index_2))) _returnvalue_2) (+ (.y (CallFunction|CoordtoActualLocation (CallFunction|IndextoCoord _array_index_2))) _returnvalue_2) (.z (CallFunction|CoordtoActualLocation (CallFunction|IndextoCoord _array_index_2)))) "0, 0, 0" "1,1,1") "Undefined" 0 (CallFunction|IndextoCoord _array_index_2) 0))
        (Utilities|Array|Add (Variables|Default|GetUnitArray) _returnvalue_8)))))

(fn Click
  (params (Position :type Vector))
  (bind _returnvalue (Transformation|GetActorLocation))
  (bind _tilesize (Variables|Default|GetTileSize))
  (bind _tilesize_2 (Variables|Default|GetTileSize))
  (bind _returnvalue_2 (- Position _returnvalue))
  (bind _returnvalue_3 (/ _tilesize_2 2))
  (bind _returnvalue_4 (Math|Conversions|ToFloat(Integer) _tilesize))
  (bind _returnvalue_5 (/ _returnvalue_2 (Math|Vector|MakeVector _returnvalue_4 _returnvalue_4 1.0)))
  (bind _returnvalue_6 (Math|Conversions|ToFloat(Integer) _returnvalue_3))
  (bind _returnvalue_7 (Math|Float|Floor (.x _returnvalue_5)))
  (bind _returnvalue_8 (Math|Float|Floor (.y _returnvalue_5)))
  (Development|PrintString (Utilities|String|BuildString(Integer) (Utilities|String|ToString(Integer) _returnvalue_7) ", " _returnvalue_8))
  (Variables|Default|SetNew%20Click (Utilities|Struct|MakeCoord _returnvalue_7 _returnvalue_8))
  (if (and (== (.x (Variables|Default|GetPreviously%20Selected)) -1) (== (.y (Variables|Default|GetPreviously%20Selected)) -1))
    ;[1 1 1] When Nothing is selected, look for unit
    (for _array_element (Variables|Default|GetUnitArray)
      (if (and (== (.x (Variables|Default|GetNew%20Click)) (.x (Variables|/Game/Blueprints/BP_Unit.BP_Unit_C|GetCoord _array_element))) (== (.y (Variables|Default|GetNew%20Click)) (.y (Variables|/Game/Blueprints/BP_Unit.BP_Unit_C|GetCoord _array_element))))
        (Variables|Default|SetPreviously%20Selected (Variables|Default|GetNew%20Click))
        (Development|PrintString "somethign is selected")))
    (else
      ;[1 1 1] Find the tile
      (for _array_element_2 (Variables|Default|GetTileArray)
        (if (and (== (.x (Variables|Default|GetNew%20Click)) (.x (Variables|/Game/Blueprints/BP_Tile.BP_Tile_C|GetCoord _array_element_2))) (== (.y (Variables|Default|GetNew%20Click)) (.y (Variables|/Game/Blueprints/BP_Tile.BP_Tile_C|GetCoord _array_element_2))))
          ;[1 1 1] See if the unit can be placed there
          (if (Variables|/Game/Blueprints/BP_Tile.BP_Tile_C|GetIsPlaceable _array_element_2)
            ;[1 1 1] make sure there isnt already a unit there
            (for _array_element_3 (Variables|Default|GetUnitArray)
              (if (and (== (.x (Variables|Default|GetNew%20Click)) (.x (Variables|/Game/Blueprints/BP_Unit.BP_Unit_C|GetCoord _array_element_3))) (== (.y (Variables|Default|GetNew%20Click)) (.y (Variables|/Game/Blueprints/BP_Unit.BP_Unit_C|GetCoord _array_element_3))))
                (Variables|Default|SetIsOccupied true)))
            (if (Variables|Default|GetIsOccupied)
              (Development|PrintString "This is already occupied")
              (Variables|Default|SetIsOccupied false)
              (else
                (for _array_element_4 (Variables|Default|GetUnitArray)
                  (if (and (== (.x (Variables|Default|GetPreviously%20Selected)) (.x (Variables|/Game/Blueprints/BP_Unit.BP_Unit_C|GetCoord _array_element_4))) (== (.y (Variables|Default|GetPreviously%20Selected)) (.y (Variables|/Game/Blueprints/BP_Unit.BP_Unit_C|GetCoord _array_element_4))))
                    (Utilities|FlowControl|Sequence
                      (:then_0
                        ;[1 1 1] move unit on the board
                        (Transformation|SetActorLocation _array_element_4 (Math|Vector|MakeVector (+ (.x (CallFunction|CoordtoActualLocation (Variables|Default|GetNew%20Click))) _returnvalue_6) (+ (.y (CallFunction|CoordtoActualLocation (Variables|Default|GetNew%20Click))) _returnvalue_6) (.z (CallFunction|CoordtoActualLocation (Variables|Default|GetNew%20Click)))) false false))
                      (:then_1
                        ;[1 1 1] Change the Coord of the unit, so the unit knows where it is
                        (bind _asbp_unit (Utilities|Casting|CastToBP_Unit _array_element_4))
                        (Variables|/Game/Blueprints/BP_Unit.BP_Unit_C|SetCoord _asbp_unit (Variables|Default|GetNew%20Click)))
                      (:then_2
                        ;[1 1 1] Reset What is Selected
                        (Variables|Default|SetPreviously%20Selected (Utilities|Struct|MakeCoord -1 -1))
                        ;[1 1 1] This probably doesnt matter
                        (Variables|Default|SetNew%20Click (Utilities|Struct|MakeCoord -1 -1))))))))
            (else
              (Development|PrintString "Unit cannot be moved there"))))))))

(fn ClearMap
  (bind _tilearray (Variables|Default|GetTileArray))
  (bind _unitarray (Variables|Default|GetUnitArray))
  (Development|PrintString "Resetting Map")
  ;[1 1 1] Clearing old Board
  (for _array_element _tilearray
    (Actor|DestroyActor _array_element))
  (Utilities|Array|Clear _tilearray)
  (for _array_element_2 _unitarray
    (Actor|DestroyActor _array_element_2))
  (Utilities|Array|Clear _unitarray))

(fn CoordtoActualLocation
  (params (Coord :type Coord%20Structure))
  (bind _returnvalue (Transformation|GetActorLocation))
  (bind _tilesize (Variables|Default|GetTileSize))
  (return (Math|Vector|MakeVector (+ (.x _returnvalue) (Math|Conversions|ToFloat(Integer) (* (.x Coord) _tilesize))) (+ (.y _returnvalue) (Math|Conversions|ToFloat(Integer) (* (.y Coord) _tilesize))) (.z _returnvalue))))

(fn ActualLocationtoCoord
  (params (Actual%20Location :type Vector))
  (bind _returnvalue (Transformation|GetActorLocation))
  (bind _tilesize (Variables|Default|GetTileSize))
  (bind _returnvalue_2 (- Actual%20Location _returnvalue))
  (bind _returnvalue_3 (Math|Conversions|ToFloat(Integer) _tilesize))
  (bind _returnvalue_4 (/ _returnvalue_2 (Math|Vector|MakeVector _returnvalue_3 _returnvalue_3 1.0)))
  (return (Utilities|Struct|MakeCoord (Math|Float|Floor (.x _returnvalue_4)) (Math|Float|Floor (.y _returnvalue_4)))))